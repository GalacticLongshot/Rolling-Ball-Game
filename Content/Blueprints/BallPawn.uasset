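; BallPawn is a player-controlled rolling ball pawn that moves and jumps through physics on its BallMesh.
; MoveForward and MoveRight axis inputs apply scaled torque as acceleration change on world Y and X to roll the ball.
; Jump adds an upward velocity-change impulse only while CanJump is set, then clears it.
; Any Hit event re-enables jumping, so wall contacts also restore the jump.
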(event `InputAxis|MoveForward`
  (params (AxisValue :type "Float (single-precision)"))
  ;[1 1 1] Move The Ball
  (`PrimitiveComponent.AddTorqueInDegrees` (`self.BallMesh`) (`KismetMathLibrary.MakeVector` 0.0 (* AxisValue (`self.Torque`))) "None" true))

(event `InputAxis|MoveRight`
  (params (AxisValue :type "Float (single-precision)"))
  ;[1 1 1] Move The Ball
  (`PrimitiveComponent.AddTorqueInDegrees` (`self.BallMesh`) (`KismetMathLibrary.MakeVector` (* AxisValue (`self.Torque`) -1.0)) "None" true))

(event `InputAction|Jump`
  (params (Key :type "Key Structure"))
  (:`Pressed`
    (if (`self.CanJump`)
      (`PrimitiveComponent.AddImpulse` (`self.BallMesh`) (`KismetMathLibrary.MakeVector` 0.0 0.0 (`self.Impulse`)) "None" true)
      (set `self.CanJump` false))))

(event `self.ReceiveHit`
  (params (MyComp :type "PrimitiveComponent Object Reference") (Other :type "Actor Object Reference") (OtherComp :type "PrimitiveComponent Object Reference") (bSelfMoved :type Boolean) (HitLocation :type "Vector Structure") (HitNormal :type "Vector Structure") (NormalImpulse :type "Vector Structure") (Hit :type "HitResult Structure (by ref)"))
  (set `self.CanJump` true))

(fn `UserConstructionScript`)